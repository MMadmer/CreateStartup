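; NPC spawner that periodically spawns a chosen class and moves each NPC along its spline.
; A self-restarting timer with random delays spawns NPCs, and the spawner attaches itself to the first BP_CSGameMap found.
; Tick advances each NPC's stored spline distance using the class-default speed, destroying those past the end and pruning invalid entries afterwards.
; MakeBox sizes the Box component from a temporary spawn's skeletal mesh bounds.
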(event Custom|MakeBox
  (bind _spawnclass (Variables|Default|GetSpawnClass))
  (if (Utilities|IsValidClass _spawnclass)
    (bind _returnvalue (Game|SpawnActorfromClass _spawnclass (Transformation|GetActorTransform) "AlwaysSpawn" 0 0))
    (Components|Box|SetBoxExtent (Variables|Default|GetBox) (.boxextent (StaticMesh|GetBounds (Variables|/Script/Engine.SkinnedMeshComponent|GetSkeletalMesh (Variables|/Script/CreateStartup.CSNPC|GetSkeletalMeshComponent _returnvalue)))) false)
    (Actor|DestroyActor _returnvalue)))

(event Custom|SpawnInit
  (CallFunction|Spawn)
  (Utilities|Time|SetTimerbyEvent (delegate Custom|SpawnInit) (Math|Random|RandomFloatinRange (Variables|SpawnerSettings|GetMinSpawnDelay) (Variables|SpawnerSettings|GetMaxSpawnDelay))))

(event EventBeginPlay
  (Utilities|Time|SetTimerbyEvent (delegate Custom|SpawnInit) (Math|Random|RandomFloatinRange (Variables|SpawnerSettings|GetMinSpawnDelay) (Variables|SpawnerSettings|GetMaxSpawnDelay)))
  (Variables|Spawnersettings|SetNPCSpeed (Utilities|GetClassDefaults (Variables|Default|GetSpawnClass)))
  (bind _outactors (Actor|GetAllActorsOfClass "/Game/CreateStartup/GameLogic/Blueprints/GameObjects/BP_CSGameMap.BP_CSGameMap_C"))
  (if (Utilities|Array|IsValidIndex _outactors)
    (Transformation|AttachActorToActor (Utilities|Array|Get(acopy) _outactors) "None" "KeepWorld" "KeepWorld" "KeepWorld" false)))

(event EventTick
  (params (DeltaSeconds :type Float%20%28single-precision%29))
  (bind _npctodestroy (Variables|Default|GetNPCToDestroy))
  (for (_array_element _array_index) (Variables|Default|GetSpawnedNPC)
    (Utilities|IsValid (.NPC (Utilities|Struct|BreakF_SpawnerInfo _array_element))
      (:Is%20Valid
        (bind (_endlocation _npc) (CallFunction|MoveNPC _array_element))
        (Utilities|Array|SetArrayElem (Variables|Default|GetSpawnedNPC) _array_index _npc)
        (if _endlocation
          (Actor|DestroyActor (.NPC (Utilities|Struct|BreakF_SpawnerInfo _array_element)))
          (Utilities|Array|Add (Variables|Default|GetNPCToDestroy) _array_element :!label _label)))
      (:Is%20Not%20Valid
        (goto _label))))
  (for _array_element_2 _npctodestroy
    (Utilities|Array|RemoveItem (Variables|Default|GetSpawnedNPC) _array_element_2))
  (Utilities|Array|Clear _npctodestroy))

(fn ConstructionScript
  (Variables|SpawnerSettings|SetMaxSpawnDelay (Math|Float|Max(Float) (Variables|SpawnerSettings|GetMinSpawnDelay) (Variables|SpawnerSettings|GetMaxSpawnDelay))))

(fn Spawn
  (bind _returnvalue (Transformation|GetActorTransform))
  (bind _spawnclass (Variables|Default|GetSpawnClass))
  (if (Utilities|IsValidClass _spawnclass)
    (bind _returnvalue_2 (Game|SpawnActorfromClass _spawnclass (Math|Transform|MakeTransform (.location _returnvalue) (.rotation _returnvalue) (.scale _returnvalue)) "AlwaysSpawn" self 0))
    (Utilities|Array|Add (Variables|Default|GetSpawnedNPC) (Utilities|Struct|MakeF_SpawnerInfo _returnvalue_2 0.0))))

(fn MoveNPC
  (params (NPCInfo :type F%20Spawner%20Info%20Structure%20%28by%20ref%29))
  (bind _output_get (LocalVariables|SetNewLocation (+ (.currentdist NPCInfo) (* (Utilities|Time|GetWorldDeltaSeconds) (Variables|Spawnersettings|GetNPCSpeed)))))
  (if (<= _output_get (Spline|GetSplineLength (Variables|Default|GetSpline)))
    (Transformation|SetActorTransform (.npc NPCInfo) (Math|Transform|MakeTransform (.location (Spline|GetTransformatDistanceAlongSpline (Variables|Default|GetSpline) (LocalVariables|GetNewLocation) "World" false)) (.rotation (Spline|GetTransformatDistanceAlongSpline (Variables|Default|GetSpline) (LocalVariables|GetNewLocation) "World" false)) (Transformation|GetActorScale3D (.npc NPCInfo))) false true)
    (LocalVariables|SetInfo (Utilities|Struct|MakeF_SpawnerInfo (.npc NPCInfo) (LocalVariables|GetNewLocation)))
    (else
      (LocalVariables|SetEnd true)
      (LocalVariables|SetInfo NPCInfo)))
  (return (LocalVariables|GetEnd) (LocalVariables|GetInfo)))
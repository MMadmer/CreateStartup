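; BP_CSNPC_Human is a human NPC Blueprint that gives itself a randomly chosen look and looping animation on BeginPlay.
; It picks a random index into the MeshVariations map, whose keys supply skeletal meshes and values supply animation sequences.
; Both assets are loaded with blocking loads, then applied to SkeletalMeshMain, which plays the animation directly.
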(event EventBeginPlay
  (bind _keys (Utilities|Map|Keys (Variables|Default|GetMeshVariations)))
  (Variables|Default|SetRandomElem (.OutIndex (Utilities|Array|Random _keys)))
  (bind _values (Utilities|Map|Values (Variables|Default|GetMeshVariations)))
  (bind _returnvalue (Utilities|LoadAssetBlocking (Utilities|Array|Get(acopy) _keys (Variables|Default|GetRandomElem))))
  (bind _returnvalue_2 (Utilities|LoadAssetBlocking (Utilities|Array|Get(acopy) _values (Variables|Default|GetRandomElem))))
  (bind _asskeletal_mesh (Utilities|Casting|CastToSkeletalMesh _returnvalue))
  (Class|SkinnedMeshComponent|SetSkeletalMesh (Variables|Default|GetSkeletalMeshMain) _asskeletal_mesh true)
  (bind _asanim_sequence (Utilities|Casting|CastToAnimSequence _returnvalue_2))
  (Components|Animation|SetAnimation (Variables|Default|GetSkeletalMeshMain) _asanim_sequence)
  (Components|Animation|PlayAnimation (Variables|Default|GetSkeletalMeshMain) _asanim_sequence true))

(fn ConstructionScript)
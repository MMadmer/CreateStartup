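; BP_CSPlayerController is the player controller that relays HUD interactions to the game's AR and audio subsystems.
; On BeginPlay it casts the HUD to BP_CSHUD and binds handlers to its scan start, scan stop and ambient volume events.
; Scan events toggle the active scan state on the AR subsystem, and volume changes pass a normalized value to the audio subsystem as ambient volume.
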(event Custom|OnStartScanning
  (Class|CSARSubsystem|SetIsScanActive (Subsystems|GetCSARSubsystem) true))

(event Custom|OnStopScanning
  (Class|CSARSubsystem|SetIsScanActive (Subsystems|GetCSARSubsystem) false))

(event Custom|OnAmbientVolumeChanged
  (params (VolumeNorm :type Float%20%28single-precision%29))
  (Class|CSAudioSubsystem|SetAmbientVolume (Subsystems|GetCSAudioSubsystem) VolumeNorm))

(event EventBeginPlay
  (bind _asbp_cshud (Utilities|Casting|CastToBP_CSHUD (HUD|GetHUD)))
  (EventDispatchers|AssignOnStartScanning _asbp_cshud (delegate Custom|OnStartScanning))
  (EventDispatchers|AssignOnStopScanning _asbp_cshud (delegate Custom|OnStopScanning))
  (EventDispatchers|AssignOnAmbientVolumeChanged _asbp_cshud (delegate Custom|OnAmbientVolumeChanged)))

(fn ConstructionScript)
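; BP_CSPlayerState is a player state Blueprint that holds the player's money balance.
; It exposes functions to read the balance, add to it, and remove from it only when funds suffice, with removal returning whether it succeeded.
; AddPlayerMoney always returns false, and the event graph and construction script are empty.
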(event EventBeginPlay)

(event EventTick
  (params (DeltaSeconds :type Float%20%28single-precision%29)))

(fn ConstructionScript)

(fn AddPlayerMoney
  (params (Money :type Integer))
  (Variables|Default|SetPlayerMoney (+ (Variables|Default|GetPlayerMoney) Money))
  (return false))

(fn GetPlayerMoney
  (return (Variables|Default|GetPlayerMoney)))

(fn RemovePlayerMoney
  (params (Money :type Integer))
  (if (>= (Variables|Default|GetPlayerMoney) Money)
    (Variables|Default|SetPlayerMoney (- (Variables|Default|GetPlayerMoney) Money))
    (return true)
    (else
      (return false))))
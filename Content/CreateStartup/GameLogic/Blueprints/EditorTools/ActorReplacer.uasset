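; Editor utility actor that swaps placed StaticMeshActors for Blueprint actors based on their mesh, and destroys itself on BeginPlay.
; ReplaceAllMeshes looks up each actor's mesh in the MeshesToReplace map and spawns the mapped class at the same transform.
; Replacements implementing CSEditorTools receive the original mesh via SetMeshMessage before the source actor is destroyed.
; Entries mapped to StaticMeshActor itself are skipped with a printed notice.
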(event Custom|ReplaceAllMeshes
  (bind _outactors (Actor|GetAllActorsOfClass "/Script/Engine.StaticMeshActor"))
  (for _array_element _outactors
    (if (.ReturnValue (Utilities|Map|Find (Variables|Default|GetMeshesToReplace) (Variables|/Script/Engine.StaticMeshComponent|GetStaticMesh (Variables|/Script/Engine.StaticMeshActor|GetStaticMeshComponent _array_element))))
      (if (not (== (.Value (Utilities|Map|Find (Variables|Default|GetMeshesToReplace) (Variables|/Script/Engine.StaticMeshComponent|GetStaticMesh (Variables|/Script/Engine.StaticMeshActor|GetStaticMeshComponent _array_element)))) "/Script/Engine.StaticMeshActor"))
        (bind _returnvalue (Game|SpawnActorfromClass (.Value (Utilities|Map|Find (Variables|Default|GetMeshesToReplace) (Variables|/Script/Engine.StaticMeshComponent|GetStaticMesh (Variables|/Script/Engine.StaticMeshActor|GetStaticMeshComponent _array_element)))) (Transformation|GetActorTransform _array_element) "AlwaysSpawn" 0 0))
        (Utilities|IsImplementInterface _returnvalue "/Script/CreateStartup.CSEditorTools"
          (:True
            (Class|CSEditorTools|SetMesh(Message) _returnvalue (Variables|/Script/Engine.StaticMeshComponent|GetStaticMesh (Variables|/Script/Engine.StaticMeshActor|GetStaticMeshComponent _array_element)))
            (Actor|DestroyActor _array_element))
          (:False
            (Actor|DestroyActor _array_element)))
        (else
          (Development|PrintString "Already is static mesh actor" true true "(R=0.000000,G=0.660000,B=1.000000,A=1.000000)" 5.0))))))

(event EventBeginPlay
  (Actor|DestroyActor))

(fn ConstructionScript)
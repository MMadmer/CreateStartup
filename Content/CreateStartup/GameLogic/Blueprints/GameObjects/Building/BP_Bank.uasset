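; Bank building actor that opens a banking screen on touch or click, letting the player manage money, cashback and savings.
; BeginPlay creates a hidden WBP_Bank widget and binds its dispatchers to handlers for a fixed cash grant, adjustable repayments and deposits, and payouts.
; Money and cashback go through interface messages on the PlayerState, whose ChangeMoney event refreshes the balance display.
; The savings balance lives on this actor.
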(event Custom|ClickOnBank
  (Input|SetInputModeUIOnly (Game|GetPlayerController 0) 0 "DoNotLock")
  (Widget|SetVisibility (Variables|Default|GetWBP_Bank) "Visible")
  (Utilities|IsImplementInterface (Variables|/Script/Engine.Controller|GetPlayerState (Game|GetPlayerController 0)) "/Game/CreateStartup/GameLogic/Blueprints/Interfaces/BPI_Stats.BPI_Stats_C"
    (:True
      (CallFunction|ViewCashbackBalance))))

(event Custom|OnTouch
  (params (FingerIndex :type ETouchIndex%20Enum :default "Touch1") (TouchedActor :type Actor%20Object%20Reference))
  (Input|SetInputModeUIOnly (Game|GetPlayerController 0) 0 "DoNotLock")
  (Widget|SetVisibility (Variables|Default|GetWBP_Bank) "Visible")
  (Utilities|IsImplementInterface (Variables|/Script/Engine.Controller|GetPlayerState (Game|GetPlayerController 0)) "/Game/CreateStartup/GameLogic/Blueprints/Interfaces/BPI_Stats.BPI_Stats_C"
    (:True
      (CallFunction|ViewCashbackBalance))))

(event Custom|OnSavingPlus
  (Variables|Default|SetSavingValue (+ (Variables|Default|GetSavingValue) 100))
  (CallFunction|ViewSavingValue))

(event Custom|OnSavingMinus
  (if (>= (Variables|Default|GetSavingValue) 101)
    (Variables|Default|SetSavingValue (- (Variables|Default|GetSavingValue) 100))
    (CallFunction|ViewSavingValue)))

(event Custom|clickmenu
  (bind _returnvalue (UserInterface|CreateWidget "/Game/CreateStartup/GameLogic/Blueprints/UserInterface/InGame/WBP_MainMenu.WBP_MainMenu_C"))
  (UserInterface|Viewport|AddtoViewport _returnvalue 0))

(event Custom|OnAddSavingBalance
  (Class|BPIStats|AddPlayerMoney(Message) (Variables|/Script/Engine.Controller|GetPlayerState (Game|GetPlayerController 0)) (Variables|Default|GetSavingsBalance))
  (Variables|Default|SetSavingsBalance 0)
  (CallFunction|ViewSavingsBalance))

(event Custom|OnBankClose
  (Widget|SetVisibility (Variables|Default|GetWBP_Bank) "Hidden")
  (Input|SetInputModeGameandUI (Game|GetPlayerController 0) 0 "DoNotLock" true))

(event Custom|OnAddMoney
  (bind _wbp_bank (Variables|Default|GetWBP_Bank))
  (Class|BPIStats|AddPlayerMoney(Message) (Variables|/Script/Engine.Controller|GetPlayerState (Game|GetPlayerController 0)) 10000)
  (Widget|SetIsEnabled (Variables|/Game/CreateStartup/GameLogic/Blueprints/UserInterface/InGame/WBP_Bank.WBP_Bank_C|Getadd_money _wbp_bank) false)
  (Widget|SetIsEnabled (Variables|/Game/CreateStartup/GameLogic/Blueprints/UserInterface/InGame/WBP_Bank.WBP_Bank_C|Getremove_money _wbp_bank) true))

(event Custom|OnRemoveMoney
  (Class|BPIStats|RemovePlayerMoney(Message) (Variables|/Script/Engine.Controller|GetPlayerState (Game|GetPlayerController 0)) (Variables|Default|GetMoneyValue)))

(event Custom|OnAddCashbackBalance
  (bind _returnvalue (Game|GetPlayerController 0))
  (bind _playerstate (Variables|/Script/Engine.Controller|GetPlayerState _returnvalue))
  (bind _cashback (Class|BPIStats|GetCashback(Message) _playerstate))
  (Class|BPIStats|AddPlayerMoney(Message) _playerstate _cashback)
  (Class|BPIStats|RemoveCashback(Message) _playerstate _cashback)
  (CallFunction|ViewCashbackBalance))

(event Custom|ChangeMoney_Event_1
  (CallFunction|ViewBalans))

(event Custom|OnRemoveSavingBalance
  (bind _savingvalue (Variables|Default|GetSavingValue))
  (bind _success (Class|BPIStats|RemovePlayerMoney(Message) (Variables|/Script/Engine.Controller|GetPlayerState (Game|GetPlayerController 0)) _savingvalue))
  (if _success
    (Variables|Default|SetSavingsBalance (+ (Variables|Default|GetSavingsBalance) _savingvalue))
    (CallFunction|ViewSavingsBalance)))

(event Custom|OnMoneyPlus
  (Variables|Default|SetMoneyValue (+ (Variables|Default|GetMoneyValue) 100))
  (CallFunction|ViewMoneyValue))

(event Custom|OnMoneyMinus
  (if (>= (Variables|Default|GetMoneyValue) 101)
    (Variables|Default|SetMoneyValue (- (Variables|Default|GetMoneyValue) 100))
    (CallFunction|ViewMoneyValue)))

(event EventBeginPlay
  (bind _returnvalue (UserInterface|CreateWidget "/Game/CreateStartup/GameLogic/Blueprints/UserInterface/InGame/WBP_Bank.WBP_Bank_C"))
  (bind _output_get (Variables|Default|SetWBP_Bank _returnvalue))
  (UserInterface|Viewport|AddtoViewport _output_get 0)
  (Widget|SetVisibility _output_get "Hidden")
  (EventDispatchers|AssignOnInputTouchBegin (delegate Custom|OnTouch))
  (CallFunction|ViewBalans)
  (CallFunction|ViewCashbackBalance)
  (CallFunction|ViewSavingsBalance)
  (bind _asbp_csplayer_state (Utilities|Casting|CastToBP_CSPlayerState (Variables|/Script/Engine.Controller|GetPlayerState (Game|GetPlayerController 0))))
  (EventDispatchers|AssignChangeMoney _asbp_csplayer_state (delegate Custom|ChangeMoney_Event_1))
  (EventDispatchers|AssignOnCloseBank (Variables|Default|GetWBP_Bank) (delegate Custom|OnBankClose))
  (EventDispatchers|AssignOnAddMoney (Variables|Default|GetWBP_Bank) (delegate Custom|OnAddMoney))
  (EventDispatchers|AssignOnRemoveMoney (Variables|Default|GetWBP_Bank) (delegate Custom|OnRemoveMoney))
  (EventDispatchers|AssignOnAddCashbackBalance (Variables|Default|GetWBP_Bank) (delegate Custom|OnAddCashbackBalance))
  (EventDispatchers|AssignOnAddSavingBalance (Variables|Default|GetWBP_Bank) (delegate Custom|OnAddSavingBalance))
  (EventDispatchers|AssignOnRemoveSavingBalance (Variables|Default|GetWBP_Bank) (delegate Custom|OnRemoveSavingBalance))
  (EventDispatchers|AssignOnMoneyPlus (Variables|Default|GetWBP_Bank) (delegate Custom|OnMoneyPlus))
  (EventDispatchers|AssignOnMoneyMinus (Variables|Default|GetWBP_Bank) (delegate Custom|OnMoneyMinus))
  (EventDispatchers|AssignOnSavingPlus (Variables|Default|GetWBP_Bank) (delegate Custom|OnSavingPlus))
  (EventDispatchers|AssignOnSavingMinus (Variables|Default|GetWBP_Bank) (delegate Custom|OnSavingMinus)))

(event EventSetMesh
  (params (NewMesh :type Static%20Mesh%20Object%20Reference))
  (Components|StaticMesh|SetStaticMesh (Variables|Default|GetStaticMesh) NewMesh))

(fn ConstructionScript)

(fn ViewBalans
  (bind _money (Class|BPIStats|GetPlayerMoney(Message) (Variables|/Script/Engine.Controller|GetPlayerState (Game|GetPlayerController 0))))
  (Variables|Default|SetPlayerMoney _money)
  (Rendering|Components|TextRender|SetText (Variables|/Game/CreateStartup/GameLogic/Blueprints/UserInterface/InGame/WBP_Bank.WBP_Bank_C|GetPlayerMoney (Variables|Default|GetWBP_Bank)) (Utilities|Text|ToText(Integer) _money)))

(fn ViewCashbackBalance
  (bind _cashback (Class|BPIStats|GetCashback(Message) (Variables|/Script/Engine.Controller|GetPlayerState (Game|GetPlayerController 0))))
  (Rendering|Components|TextRender|SetText (Variables|/Game/CreateStartup/GameLogic/Blueprints/UserInterface/InGame/WBP_Bank.WBP_Bank_C|GetCashbackBalance (Variables|Default|GetWBP_Bank)) (Utilities|Text|ToText(Integer) _cashback)))

(fn ViewSavingsBalance
  (Rendering|Components|TextRender|SetText (Variables|/Game/CreateStartup/GameLogic/Blueprints/UserInterface/InGame/WBP_Bank.WBP_Bank_C|GetSavingsBalance (Variables|Default|GetWBP_Bank)) (Utilities|Text|ToText(Integer) (Variables|Default|GetSavingsBalance))))

(fn ViewMoneyValue
  (Rendering|Components|TextRender|SetText (Variables|/Game/CreateStartup/GameLogic/Blueprints/UserInterface/InGame/WBP_Bank.WBP_Bank_C|GetMoneyValue (Variables|Default|GetWBP_Bank)) (Utilities|Text|ToText(Integer) (Variables|Default|GetMoneyValue))))

(fn ViewSavingValue
  (Rendering|Components|TextRender|SetText (Variables|/Game/CreateStartup/GameLogic/Blueprints/UserInterface/InGame/WBP_Bank.WBP_Bank_C|GetSavingValue (Variables|Default|GetWBP_Bank)) (Utilities|Text|ToText(Integer) (Variables|Default|GetSavingValue))))

(fn GetMesh
  (return (Variables|/Script/Engine.StaticMeshComponent|GetStaticMesh (Variables|Default|GetStaticMesh))))

(fn Click
  (return false))
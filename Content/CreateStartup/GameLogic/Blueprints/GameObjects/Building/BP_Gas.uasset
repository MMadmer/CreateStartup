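; BP_Gas is a building actor that opens the WBP_Gas screen when it is tapped or clicked.
; BeginPlay creates the widget hidden, binds touch input and listens to the widget's exit dispatcher.
; Touch and ClickOnGas share one path that shows the widget in UI-only input, and exit hides it and restores game-and-UI input.
; A BPI_Stats interface check on the PlayerState ends that path with its result unused.
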(event Custom|ClickOnGas
  (Input|SetInputModeUIOnly (Game|GetPlayerController 0) 0 "DoNotLock")
  (Widget|SetVisibility (Variables|Default|Getwbp_gas) "Visible")
  (Utilities|IsImplementInterface (Variables|/Script/Engine.Controller|GetPlayerState (Game|GetPlayerController 0)) "/Game/CreateStartup/GameLogic/Blueprints/Interfaces/BPI_Stats.BPI_Stats_C"))

(event Custom|OnTouch
  (params (FingerIndex :type ETouchIndex%20Enum :default "Touch1") (TouchedActor :type Actor%20Object%20Reference))
  (Input|SetInputModeUIOnly (Game|GetPlayerController 0) 0 "DoNotLock")
  (Widget|SetVisibility (Variables|Default|Getwbp_gas) "Visible")
  (Utilities|IsImplementInterface (Variables|/Script/Engine.Controller|GetPlayerState (Game|GetPlayerController 0)) "/Game/CreateStartup/GameLogic/Blueprints/Interfaces/BPI_Stats.BPI_Stats_C"))

(event Custom|ExitDisptcher_Event_0
  (Widget|SetVisibility (Variables|Default|Getwbp_gas) "Hidden")
  (Input|SetInputModeGameandUI (Game|GetPlayerController 0) 0 "DoNotLock" true))

(event EventBeginPlay
  (bind _returnvalue (UserInterface|CreateWidget "/Game/CreateStartup/GameLogic/Blueprints/UserInterface/InGame/WBP_Gas.WBP_Gas_C"))
  (bind _output_get (Variables|Default|Setwbp_gas _returnvalue))
  (UserInterface|Viewport|AddtoViewport _output_get 0)
  (Widget|SetVisibility _output_get "Hidden")
  (EventDispatchers|AssignOnInputTouchBegin (delegate Custom|OnTouch))
  (EventDispatchers|AssignExitDisptcher (Variables|Default|Getwbp_gas) (delegate Custom|ExitDisptcher_Event_0)))

(fn ConstructionScript)
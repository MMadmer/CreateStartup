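; BP_Storage is a storage building that opens a UI showing cost and stored-versus-maximum amounts for five candy types, plus the player's money.
; BeginPlay creates a hidden WBP_Storage widget and binds touch, exit and money-change events.
; Touch or ClickOnStorage switches to UI-only input, shows the widget and fills its text.
; Money changes refresh the balance, and exiting hides the widget and restores game-and-UI input.
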(event Custom|ClickOnStorage
  (Input|SetInputModeUIOnly (Game|GetPlayerController 0) 0 "DoNotLock")
  (Widget|SetVisibility (Variables|Default|GetStorage) "Visible")
  (CallFunction|VeiwCostandStorage)
  (CallFunction|ViewPlayerMoney)
  (Utilities|ImplementsInterface (Variables|/Script/Engine.Controller|GetPlayerState (Game|GetPlayerController 0)) "/Game/CreateStartup/GameLogic/Blueprints/Interfaces/BPI_Stats.BPI_Stats_C"))

(event Custom|OnTouch
  (params (FingerIndex :type ETouchIndex%20Enum :default "Touch1") (TouchedActor :type Actor%20Object%20Reference))
  (Input|SetInputModeUIOnly (Game|GetPlayerController 0) 0 "DoNotLock")
  (Widget|SetVisibility (Variables|Default|GetStorage) "Visible")
  (CallFunction|VeiwCostandStorage)
  (CallFunction|ViewPlayerMoney)
  (Utilities|ImplementsInterface (Variables|/Script/Engine.Controller|GetPlayerState (Game|GetPlayerController 0)) "/Game/CreateStartup/GameLogic/Blueprints/Interfaces/BPI_Stats.BPI_Stats_C"))

(event Custom|ExitDispather_Event_1
  (Widget|SetVisibility (Variables|Default|GetStorage) "Hidden")
  (Input|SetInputModeGameandUI (Game|GetPlayerController 0) 0 "DoNotLock" true))

(event Custom|ChangeMoney_Event_1
  (CallFunction|ViewPlayerMoney))

(event EventBeginPlay
  (bind _returnvalue (UserInterface|CreateWidget "/Game/CreateStartup/GameLogic/Blueprints/UserInterface/InGame/Business/WBP_Storage.WBP_Storage_C"))
  (bind _output_get (Variables|Default|SetStorage _returnvalue))
  (UserInterface|Viewport|AddtoViewport _output_get 1)
  (Widget|SetVisibility _output_get "Hidden")
  (EventDispatchers|BindEventtoOnInputTouchEnd (delegate Custom|OnTouch))
  (EventDispatchers|AssignExitDispather (Variables|Default|GetStorage) (delegate Custom|ExitDispather_Event_1))
  (bind _asbp_csplayer_state (Utilities|Casting|CastToBP_CSPlayerState (Variables|/Script/Engine.Controller|GetPlayerState (Game|GetPlayerController 0))))
  (EventDispatchers|AssignChangeMoney _asbp_csplayer_state (delegate Custom|ChangeMoney_Event_1)))

(fn ConstructionScript)

(fn VeiwCostandStorage
  (bind _storage (Variables|Default|GetStorage))
  (bind _text (Variables|Default|GetText))
  (bind _cost (Variables|Default|GetCost))
  (bind _player_volume_storage (Variables|Default|GetPlayer_volume_storage))
  (bind _volume_storage_max (Variables|Default|GetVolume_storage_max))
  (bind _storage_2 (Variables|Default|GetStorage))
  (Rendering|Components|TextRender|SetText (Variables|/Game/CreateStartup/GameLogic/Blueprints/UserInterface/InGame/Business/WBP_Storage.WBP_Storage_C|GetText_candy_1 _storage_2) (Utilities|Text|ToText(Integer) (Utilities|Array|Get(acopy) _cost)))
  (Rendering|Components|TextRender|SetText (Variables|/Game/CreateStartup/GameLogic/Blueprints/UserInterface/InGame/Business/WBP_Storage.WBP_Storage_C|GetText_candy_2 _storage_2) (Utilities|Text|ToText(Integer) (Utilities|Array|Get(acopy) _cost 1)))
  (Rendering|Components|TextRender|SetText (Variables|/Game/CreateStartup/GameLogic/Blueprints/UserInterface/InGame/Business/WBP_Storage.WBP_Storage_C|GetText_candy_3 _storage_2) (Utilities|Text|ToText(Integer) (Utilities|Array|Get(acopy) _cost 2)))
  (Rendering|Components|TextRender|SetText (Variables|/Game/CreateStartup/GameLogic/Blueprints/UserInterface/InGame/Business/WBP_Storage.WBP_Storage_C|GetText_candy_4 _storage_2) (Utilities|Text|ToText(Integer) (Utilities|Array|Get(acopy) _cost 3)))
  (Rendering|Components|TextRender|SetText (Variables|/Game/CreateStartup/GameLogic/Blueprints/UserInterface/InGame/Business/WBP_Storage.WBP_Storage_C|GetText_candy_5 _storage_2) (Utilities|Text|ToText(Integer) (Utilities|Array|Get(acopy) _cost 4)))
  (Rendering|Components|TextRender|SetText (Variables|/Game/CreateStartup/GameLogic/Blueprints/UserInterface/InGame/Business/WBP_Storage.WBP_Storage_C|GetText_Storage_candy_1 _storage) (Utilities|Text|ToText(String) (Utilities|String|Append (Utilities|String|ToString(Integer) (Utilities|Array|Get(acopy) _player_volume_storage)) (Utilities|String|Append _text (Utilities|String|ToString(Integer) (Utilities|Array|Get(acopy) _volume_storage_max))))))
  (Rendering|Components|TextRender|SetText (Variables|/Game/CreateStartup/GameLogic/Blueprints/UserInterface/InGame/Business/WBP_Storage.WBP_Storage_C|GetText_Storage_candy_2 _storage) (Utilities|Text|ToText(String) (Utilities|String|Append (Utilities|String|ToString(Integer) (Utilities|Array|Get(acopy) _player_volume_storage 1)) (Utilities|String|Append _text (Utilities|String|ToString(Integer) (Utilities|Array|Get(acopy) _volume_storage_max 1))))))
  (Rendering|Components|TextRender|SetText (Variables|/Game/CreateStartup/GameLogic/Blueprints/UserInterface/InGame/Business/WBP_Storage.WBP_Storage_C|GetText_Storage_candy_3 _storage) (Utilities|Text|ToText(String) (Utilities|String|Append (Utilities|String|ToString(Integer) (Utilities|Array|Get(acopy) _player_volume_storage 2)) (Utilities|String|Append _text (Utilities|String|ToString(Integer) (Utilities|Array|Get(acopy) _volume_storage_max 2))))))
  (Rendering|Components|TextRender|SetText (Variables|/Game/CreateStartup/GameLogic/Blueprints/UserInterface/InGame/Business/WBP_Storage.WBP_Storage_C|GetText_Storage_candy_4 _storage) (Utilities|Text|ToText(String) (Utilities|String|Append (Utilities|String|ToString(Integer) (Utilities|Array|Get(acopy) _player_volume_storage 3)) (Utilities|String|Append _text (Utilities|String|ToString(Integer) (Utilities|Array|Get(acopy) _volume_storage_max 3))))))
  (Rendering|Components|TextRender|SetText (Variables|/Game/CreateStartup/GameLogic/Blueprints/UserInterface/InGame/Business/WBP_Storage.WBP_Storage_C|GetText_Storage_candy_5 _storage) (Utilities|Text|ToText(String) (Utilities|String|Append (Utilities|String|ToString(Integer) (Utilities|Array|Get(acopy) _player_volume_storage 4)) (Utilities|String|Append _text (Utilities|String|ToString(Integer) (Utilities|Array|Get(acopy) _volume_storage_max 4)))))))

(fn ViewPlayerMoney
  (bind _money (Class|BPIStats|GetPlayerMoney(Message) (Variables|/Script/Engine.Controller|GetPlayerState (Game|GetPlayerController 0))))
  (Rendering|Components|TextRender|SetText (Variables|/Game/CreateStartup/GameLogic/Blueprints/UserInterface/InGame/Business/WBP_Storage.WBP_Storage_C|GetPlayerMoney (Variables|Default|GetStorage)) (Utilities|Text|ToText(Integer) _money)))
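; Shop building that opens a WBP_Shop widget on touch or click, where the player buys five types of candy for storage.
; The widget is created hidden at BeginPlay, shows prices and balance, and toggles input mode when opened or closed.
; Its buy dispatchers feed BuyCandy, which checks BP_Storage capacity, charges PlayerState through interface messages, increments stock and grants cashback.
; BP_CSPlayerState's ChangeMoney dispatcher refreshes the displayed balance.
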(event Custom|ClickOnShop
  (Input|SetInputModeUIOnly (Game|GetPlayerController 0) 0 "DoNotLock")
  (Widget|SetVisibility (Variables|Default|GetShop) "Visible")
  (Utilities|IsImplementInterface (Variables|/Script/Engine.Controller|GetPlayerState (Game|GetPlayerController 0)) "/Game/CreateStartup/GameLogic/Blueprints/Interfaces/BPI_Stats.BPI_Stats_C"))

(event Custom|OnTouch
  (params (FingerIndex :type ETouchIndex%20Enum :default "Touch1") (TouchedActor :type Actor%20Object%20Reference))
  (Input|SetInputModeUIOnly (Game|GetPlayerController 0) 0 "DoNotLock")
  (Widget|SetVisibility (Variables|Default|GetShop) "Visible")
  (Utilities|IsImplementInterface (Variables|/Script/Engine.Controller|GetPlayerState (Game|GetPlayerController 0)) "/Game/CreateStartup/GameLogic/Blueprints/Interfaces/BPI_Stats.BPI_Stats_C"))

(event Custom|BuyCandy2_Event_0
  (CallFunction|BuyCandy 1))

(event Custom|ExitDispather_Event_0
  (Widget|SetVisibility (Variables|Default|GetShop) "Hidden")
  (Input|SetInputModeGameandUI (Game|GetPlayerController 0) 0 "DoNotLock" true))

(event Custom|BuyCandy1_Event_0
  (CallFunction|BuyCandy))

(event Custom|ChangeMoney_Event_1
  (CallFunction|ViewBalansPlayer))

(event Custom|BuyCandy3_Event_0
  (CallFunction|BuyCandy 2))

(event Custom|BuyCandy4_Event_0
  (CallFunction|BuyCandy 3))

(event Custom|BuyCandy5_Event_0
  (CallFunction|BuyCandy 4))

(event EventBeginPlay
  (bind _returnvalue (UserInterface|CreateWidget "/Game/CreateStartup/GameLogic/Blueprints/UserInterface/InGame/WBP_Shop.WBP_Shop_C"))
  (bind _output_get (Variables|Default|SetShop _returnvalue))
  (UserInterface|Viewport|AddtoViewport _output_get 0)
  (Widget|SetVisibility _output_get "Hidden")
  (EventDispatchers|AssignOnInputTouchBegin (delegate Custom|OnTouch))
  (EventDispatchers|AssignExitDispather (Variables|Default|GetShop) (delegate Custom|ExitDispather_Event_0))
  (CallFunction|CostCandyView)
  (CallFunction|ViewBalansPlayer)
  (bind _asbp_csplayer_state (Utilities|Casting|CastToBP_CSPlayerState (Variables|/Script/Engine.Controller|GetPlayerState (Game|GetPlayerController 0))))
  (EventDispatchers|AssignChangeMoney _asbp_csplayer_state (delegate Custom|ChangeMoney_Event_1))
  (EventDispatchers|AssignBuyCandy1 (Variables|Default|GetShop) (delegate Custom|BuyCandy1_Event_0))
  (EventDispatchers|AssignBuyCandy2 (Variables|Default|GetShop) (delegate Custom|BuyCandy2_Event_0))
  (EventDispatchers|AssignBuyCandy3 (Variables|Default|GetShop) (delegate Custom|BuyCandy3_Event_0))
  (EventDispatchers|AssignBuyCandy4 (Variables|Default|GetShop) (delegate Custom|BuyCandy4_Event_0))
  (EventDispatchers|AssignBuyCandy5 (Variables|Default|GetShop) (delegate Custom|BuyCandy5_Event_0)))

(fn ConstructionScript)

(fn CostCandyView
  (bind _shop (Variables|Default|GetShop))
  (bind _cost_candy (Variables|Default|GetCost_candy))
  (Rendering|Components|TextRender|SetText (Variables|/Game/CreateStartup/GameLogic/Blueprints/UserInterface/InGame/WBP_Shop.WBP_Shop_C|GetText_candy_1 _shop) (Utilities|Text|ToText(Integer) (Utilities|Array|Get(acopy) _cost_candy)))
  (Rendering|Components|TextRender|SetText (Variables|/Game/CreateStartup/GameLogic/Blueprints/UserInterface/InGame/WBP_Shop.WBP_Shop_C|GetText_candy_2 _shop) (Utilities|Text|ToText(Integer) (Utilities|Array|Get(acopy) _cost_candy 1)))
  (Rendering|Components|TextRender|SetText (Variables|/Game/CreateStartup/GameLogic/Blueprints/UserInterface/InGame/WBP_Shop.WBP_Shop_C|GetText_candy_3 _shop) (Utilities|Text|ToText(Integer) (Utilities|Array|Get(acopy) _cost_candy 2)))
  (Rendering|Components|TextRender|SetText (Variables|/Game/CreateStartup/GameLogic/Blueprints/UserInterface/InGame/WBP_Shop.WBP_Shop_C|GetText_candy_4 _shop) (Utilities|Text|ToText(Integer) (Utilities|Array|Get(acopy) _cost_candy 3)))
  (Rendering|Components|TextRender|SetText (Variables|/Game/CreateStartup/GameLogic/Blueprints/UserInterface/InGame/WBP_Shop.WBP_Shop_C|GetText_candy_5 _shop) (Utilities|Text|ToText(Integer) (Utilities|Array|Get(acopy) _cost_candy 4))))

(fn BuyCandy
  (params (NumberCandy :type Integer) (CostCandy :type Integer))
  (bind _cost_candy (Variables|Default|GetCost_candy))
  (bind _output (Utilities|Array|Get(acopy) _cost_candy NumberCandy))
  (bind _returnvalue (Actor|GetActorOfClass "/Game/CreateStartup/GameLogic/Blueprints/GameObjects/Building/BP_Storage.BP_Storage_C"))
  (if (< (Utilities|Array|Get(acopy) (Variables|/Game/CreateStartup/GameLogic/Blueprints/GameObjects/Building/BP_Storage.BP_Storage_C|GetPlayer_volume_storage _returnvalue) NumberCandy) (Utilities|Array|Get(acopy) (Variables|/Game/CreateStartup/GameLogic/Blueprints/GameObjects/Building/BP_Storage.BP_Storage_C|GetVolume_storage_max _returnvalue) NumberCandy))
    (bind _success (Class|BPIStats|RemovePlayerMoney(Message) (Variables|/Script/Engine.Controller|GetPlayerState (Game|GetPlayerController 0)) _output))
    (if _success
      (Utilities|Array|SetArrayElem (Variables|/Game/CreateStartup/GameLogic/Blueprints/GameObjects/Building/BP_Storage.BP_Storage_C|GetPlayer_volume_storage _returnvalue) NumberCandy (+ (Utilities|Array|Get(acopy) (Variables|/Game/CreateStartup/GameLogic/Blueprints/GameObjects/Building/BP_Storage.BP_Storage_C|GetPlayer_volume_storage _returnvalue) NumberCandy) 1))
      (Class|BPIStats|AddCashback(Message) (Variables|/Script/Engine.Controller|GetPlayerState (Game|GetPlayerController 0)) _output))))

(fn ViewBalansPlayer
  (bind _money (Class|BPIStats|GetPlayerMoney(Message) (Variables|/Script/Engine.Controller|GetPlayerState (Game|GetPlayerController 0))))
  (Rendering|Components|TextRender|SetText (Variables|/Game/CreateStartup/GameLogic/Blueprints/UserInterface/InGame/WBP_Shop.WBP_Shop_C|GetPlayerMoney (Variables|Default|GetShop)) (Utilities|Text|ToText(Integer) _money)))
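; BP_Cleaner is a one-shot actor that clears the level of actors that are neither whitelisted nor attached to the game map.
; Shortly after BeginPlay, a timer finds the first BP_CSGameMap and gathers its attached actors.
; It then destroys every other actor whose exact class is absent from WhiteList, and finally itself.
; If no game map exists, it does nothing.
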(event Custom|Cleaning
  (bind _outactors (Actor|GetAllActorsOfClass "/Game/CreateStartup/GameLogic/Blueprints/GameObjects/BP_CSGameMap.BP_CSGameMap_C"))
  (if (Utilities|Array|IsValidIndex _outactors)
    (bind _output_get (Variables|Default|SetGameMap (Utilities|Array|Get(acopy) _outactors)))
    (Variables|Default|SetGameMapActors (Actor|GetAttachedActors _output_get true))
    (bind _outactors_2 (Actor|GetAllActorsOfClass "/Script/Engine.Actor"))
    (for _array_element _outactors_2
      (if (< (Utilities|Array|FindItem (Variables|Default|GetWhiteList) (Utilities|GetClass _array_element)) 0)
        (if (< (Utilities|Array|FindItem (Variables|Default|GetGameMapActors) _array_element) 0)
          (Actor|DestroyActor _array_element))))
    (Actor|DestroyActor)))

(event EventBeginPlay
  (Utilities|Time|SetTimerbyEvent (delegate Custom|Cleaning) 0.2))

(fn ConstructionScript)
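; BP_CSGameMap is the game map actor for an AR level, anchored in the world by a tracked image.
; On BeginPlay it registers with the CS AR subsystem for image-found callbacks, each of which teleports it to the image's location, yaw and scale.
; The first callback also runs a one-time launch that spawns the map's objects and starts level ambient audio through the CS audio subsystem.
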(event Custom|OnImageFound
  (params (FoundImage :type AR%20Tracked%20Image%20Object%20Reference))
  (bind _returnvalue (Class|ARTrackedGeometry|GetLocaltoWorldTransform FoundImage))
  (Transformation|SetActorTransform (Math|Transform|MakeTransform (.location _returnvalue) (Math|Rotator|MakeRotator 0.0 0.0 (.yaw (.rotation _returnvalue))) (.scale _returnvalue)) false true)
  (if (not (Variables|Default|GetLaunched))
    (Variables|Default|SetLaunched true)
    (CallFunction|InitialSpawn)))

(event Custom|InitialSpawn
  (Class|CSGameMap|SpawnObjects)
  (Class|CSAudioSubsystem|PlayLevelAmbient (Subsystems|GetCSAudioSubsystem) (Variables|Default|GetLevelAudio) (Variables|Default|GetLevelAmbient) 1.0))

(event EventBeginPlay
  (EventDispatchers|AssignOnTrackedImageFound (Subsystems|GetCSARSubsystem) (delegate Custom|OnImageFound)))

(fn ConstructionScript)